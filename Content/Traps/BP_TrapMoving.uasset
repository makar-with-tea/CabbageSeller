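; BP_TrapMoving is a trap that shuttles between two points and repeatedly damages the player while they overlap its collision box.
; SetCharacteristics supplies the endpoints and speed; Tick makes swept, frame-rate-dependent steps and reverses near each end.
; Overlap events start and clear a looping damage timer.
; TempSlowDown halves speed, then restores it after a buff time read from the difficulty data table according to the game mode's room difficulty.
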(event OnComponentEndOverlap(CollisionBox)
  (params (OverlappedComponent :type Primitive%20Component%20Object%20Reference) (OtherActor :type Actor%20Object%20Reference) (OtherComp :type Primitive%20Component%20Object%20Reference) (OtherBodyIndex :type Integer))
  (Utilities|Casting|CastToBP_ThirdPersonCharacter OtherActor)
  (Utilities|Time|ClearTimerbyFunctionName 0 "MyApplyDamage"))

(event OnComponentBeginOverlap(CollisionBox)
  (params (OverlappedComponent :type Primitive%20Component%20Object%20Reference) (OtherActor :type Actor%20Object%20Reference) (OtherComp :type Primitive%20Component%20Object%20Reference) (OtherBodyIndex :type Integer) (bFromSweep :type Boolean) (SweepResult :type Hit%20Result%20Structure%20%28by%20ref%29))
  (Utilities|Casting|CastToBP_ThirdPersonCharacter OtherActor)
  (Utilities|Time|SetTimerbyFunctionName 0 "MyApplyDamage" 1.0 true))

(event Custom|MyApplyDamage
  (bind _asbp_third_person_character (Utilities|Casting|CastToBP_ThirdPersonCharacter (Game|Player|GetPlayerPawn 0)))
  (Game|Damage|ApplyDamage _asbp_third_person_character 1.0 0 self))

(event Custom|SetCharacteristics
  (params (StartLocation :type Vector) (EndLocation :type Vector) (Speed :type Float%20%28double-precision%29))
  (Variables|Default|SetSpeed Speed)
  (bind _output_get (Variables|Default|SetStartLocation StartLocation))
  (bind _output_get_2 (Variables|Default|SetEndLocation EndLocation))
  (Variables|Default|SetUnitVector (Class|KismetMathLibrary|VectorNormalUnsafe (- _output_get_2 _output_get)))
  (bind _output_get_3 (Variables|Default|SetTempLocation _output_get))
  (Transformation|SetActorLocation _output_get_3 false false))

(event Custom|TempSlowDown
  (bind _output_get (Variables|Default|SetSpeed (/ (Variables|Default|GetSpeed) 2.0)))
  (bind _asbp_third_person_game_mode (Utilities|Casting|CastToBP_ThirdPersonGameMode (Game|GetGameMode)))
  (if (Variables|/Game/ThirdPerson/Blueprints/BP_ThirdPersonGameMode.BP_ThirdPersonGameMode_C|GetIsDifficultRoom _asbp_third_person_game_mode)
    (bind _returnvalue (Utilities|GetDataTableRow "/Game/RoomGenerator/DifficultyDataTable.DifficultyDataTable" "Difficult")
      (:then
        (Utilities|FlowControl|Delay (Math|Conversions|ToFloat(Integer) (.BuffTimeSeconds (Utilities|Struct|BreakDifficultyDataStruct _returnvalue))))
        (Variables|Default|SetSpeed (* _output_get 2.0))))
    (else
      (bind _returnvalue_2 (Utilities|GetDataTableRow "/Game/RoomGenerator/DifficultyDataTable.DifficultyDataTable" "Easy")
        (:then
          (Utilities|FlowControl|Delay (Math|Conversions|ToFloat(Integer) (.BuffTimeSeconds (Utilities|Struct|BreakDifficultyDataStruct _returnvalue_2))))
          (Variables|Default|SetSpeed (* _output_get 2.0)))))))

(event EventBeginPlay)

(event EventTick
  (params (DeltaSeconds :type Float%20%28single-precision%29))
  (if (< (Variables|Default|GetSpeed) (Math|Vector|Distance(Vector) (+ (Transformation|GetActorLocation) (* (Variables|Default|GetUnitVector) (Variables|Default|GetSpeed))) (Variables|Default|GetEndLocation)))
    (Transformation|SetActorLocation (+ (Transformation|GetActorLocation) (* (Variables|Default|GetUnitVector) (Variables|Default|GetSpeed))) true false)
    (else
      (bind _output_get (Variables|Default|SetTempLocation (Variables|Default|GetEndLocation)))
      (Variables|Default|SetEndLocation (Variables|Default|GetStartLocation))
      (Variables|Default|SetStartLocation _output_get)
      (Variables|Default|SetUnitVector (* (Variables|Default|GetUnitVector) -1.0)))))

(fn ConstructionScript)